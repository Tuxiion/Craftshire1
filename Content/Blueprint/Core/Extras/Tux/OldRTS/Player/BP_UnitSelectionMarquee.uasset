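; Marquee selection actor for an RTS player, used to drag-select units with the cursor.
; While resizing, each tick it traces under the cursor and stretches a box collider between its own location and that point.
; Overlapping actors implementing BPI_SelectionEvents are sent to the player controller for selection, and deselected when they leave during resizing.
; Start and end functions toggle resizing and the box's query collision.
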(event `self.ReceiveTick`
  (params (DeltaSeconds :type "Float (single-precision)"))
  (bind (_returnvalue_x _returnvalue_y) (`KismetMathLibrary.BreakVector` (/ (`KismetMathLibrary.Vector_GetAbs` (- (`self.K2_GetActorLocation`) (`self.EndMouseLocation`))) 2.0)))
  (if (`self.ShouldResizeMarquee`)
    (bind _aspc_tux_rts1 (cast `/Game/Tux_RTS1/Core/Player/PC_Tux_RTS1` (`GameplayStatics.GetPlayerController` 0)))
    (bind (_bblockinghit _binitialoverlap _time _distance _location) (`GameplayStatics.BreakHitResult` (`PlayerController.GetHitResultUnderCursorByChannel` _aspc_tux_rts1 "TraceTypeQuery1" true)))
    (`SceneComponent.K2_SetWorldLocation` (`self.Sphere`) _location false false)
    (set `self.EndMouseLocation` _location)
    (`SceneComponent.K2_SetWorldLocation` (`self.BoxCol`) (`KismetMathLibrary.VLerp` (`self.K2_GetActorLocation`) (`self.EndMouseLocation`) 0.5) false false)
    (`SceneComponent.K2_SetWorldLocation` (`self.Sphere2`) (`KismetMathLibrary.VLerp` (`self.K2_GetActorLocation`) (`self.EndMouseLocation`) 0.5) false false)
    (`BoxComponent.SetBoxExtent` (`self.BoxCol`) (`KismetMathLibrary.MakeVector` _returnvalue_x _returnvalue_y 300.0) true)))

(event `self.BoxCol.OnComponentBeginOverlap`
  (params (OverlappedComponent :type "PrimitiveComponent Object Reference") (OtherActor :type "Actor Object Reference") (OtherComp :type "PrimitiveComponent Object Reference") (OtherBodyIndex :type Integer) (bFromSweep :type Boolean) (SweepResult :type "HitResult Structure (by ref)"))
  (if (`KismetSystemLibrary.DoesImplementInterface` OtherActor "/Game/Tux_RTS1/Core/Building/BPI_SelectionEvents.BPI_SelectionEvents_C")
    (message `/Game/Tux_RTS1/Core/Building/BPI_SelectionEvents.SelectThisActor` (`GameplayStatics.GetPlayerController` 0) OtherActor)))

(event `self.BoxCol.OnComponentEndOverlap`
  (params (OverlappedComponent :type "PrimitiveComponent Object Reference") (OtherActor :type "Actor Object Reference") (OtherComp :type "PrimitiveComponent Object Reference") (OtherBodyIndex :type Integer))
  (bind _shouldresizemarquee (`self.ShouldResizeMarquee`))
  (if _shouldresizemarquee
    (if (and _shouldresizemarquee (`KismetSystemLibrary.DoesImplementInterface` OtherActor "/Game/Tux_RTS1/Core/Building/BPI_SelectionEvents.BPI_SelectionEvents_C"))
      (message `/Game/Tux_RTS1/Core/Building/BPI_SelectionEvents.DeselectThisActor` (`GameplayStatics.GetPlayerController` 0) OtherActor))))

(fn `EndResizingMarquee`
  (set `self.ShouldResizeMarquee` false)
  (`PrimitiveComponent.SetCollisionEnabled` (`self.BoxCol`) "NoCollision"))

(fn `StartResizingMarquee`
  (set `self.ShouldResizeMarquee` true)
  (`PrimitiveComponent.SetCollisionEnabled` (`self.BoxCol`) "QueryOnly"))

(fn `UserConstructionScript`)